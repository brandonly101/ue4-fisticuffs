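; Fist fighter character Blueprint that manages stamina, discombobulation and melee damage for punching and blocking.
; Incoming damage drains stamina while blocking, otherwise it adds to discombobulation, which decays in one-second steps.
; Tick drains stamina while punching, regenerates it when idle, and disables both actions at empty until it refills to full.
; CharacterDealDamage applies damage to filtered actors overlapping a given collider.
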(event EventBeginPlay)

(event EventActorBeginOverlap
  (params (OtherActor :type Actor%20Object%20Reference)))

(event EventTick
  (params (DeltaSeconds :type Float%20%28single-precision%29))
  (Utilities|FlowControl|Sequence
    (:then_0
      ;[1 1 1] Degen Stamina if Punching
      (if (Variables|Default|GetPunchingToggle)
        (Variables|Default|SetStatStamina (- (Variables|Default|GetStatStamina) (Variables|Default|GetStatStaminaDegenR)))))
    (:then_1
      ;[1 1 1] Degen Discombob and Regen Stamina (Recharging)
      (Utilities|FlowControl|Sequence
        (:then_0
          (Variables|Default|SetStatDiscombobStagger (+ (Variables|Default|GetStatDiscombobStagger) (Utilities|Time|GetWorldDeltaSeconds)))
          (if (and (> (Variables|Default|GetStatDiscombobulation) 0.0) (>= (Variables|Default|GetStatDiscombobStagger) 1.0))
            (Variables|Default|SetStatDiscombobulation (- (Variables|Default|GetStatDiscombobulation) (Variables|Default|GetStatDiscombobDegenR)))
            (Variables|Default|SetStatDiscombobStagger 0.0)))
        (:then_1
          (if (Math|Boolean|ANDBoolean (< (Variables|Default|GetStatStamina) 1.0) (not (Variables|Default|GetPunchingToggle)) (not (Variables|Default|GetBlockingToggle)))
            (Variables|Default|SetStatStamina (+ (Variables|Default|GetStatStamina) (Variables|Default|GetStatStaminaRegenR)))))))
    (:then_2
      ;[1 1 1] Set Capability for Punching/Blocking
      (if (<= (Variables|Default|GetStatStamina) 0.0)
        (Variables|Default|SetPunchingCapable false)
        (Variables|Default|SetBlockingCapable false)
        (Variables|Default|SetPunchingToggle false)
        (Variables|Default|SetBlockingToggle false)
        (elif (>= (Variables|Default|GetStatStamina) 1.0)
          (Variables|Default|SetPunchingCapable true)
          (Variables|Default|SetBlockingCapable true))))))

(event EventAnyDamage
  (params (Damage :type Float%20%28single-precision%29) (DamageType :type Damage%20Type%20Object%20Reference) (InstigatedBy :type Controller%20Object%20Reference) (DamageCauser :type Actor%20Object%20Reference))
  ;[1 1 1] Take Damage
  (if (Variables|Default|GetBlockingToggle)
    (Variables|Default|SetStatStamina (- (Variables|Default|GetStatStamina) (Variables|Default|GetStatStaminaDegenR)))
    (else
      (Variables|Default|SetStatDiscombobulation (+ Damage (Variables|Default|GetStatDiscombobulation))))))

(fn ConstructionScript)

(fn CharacterDealDamage
  (params (Collider :type Sphere%20Component%20Object%20Reference) (Class%20Target%20Filter :type Actor%20Class%20Reference) (Damage :type Float%20%28single-precision%29 :default 0.0))
  (bind _output_get (LocalVariables|SetActors (Collision|GetOverlappingActors Collider Class%20Target%20Filter :!class /Script/Engine.PrimitiveComponent)))
  (for _array_element _output_get
    (Game|Damage|ApplyDamage _array_element Damage (Pawn|GetController) self))
  (Game|Damage|ApplyDamage _array_element Damage (Pawn|GetController) self))