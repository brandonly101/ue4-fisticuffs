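; BookMainMenu is a main menu actor for Fisticuffs that is visible only during the main menu state.
; Every Tick it checks the FisticuffsGameMode PlayState, showing the mouse cursor in EMainMenu and otherwise hiding itself with its children and the cursor.
; Nothing unhides it once hidden.
; A node chain to rotate it toward the player camera is present but never runs.
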(event `self.ReceiveBeginPlay`)

(event `self.ReceiveActorBeginOverlap`
  (params (OtherActor :type "Actor Object Reference")))

(event `self.ReceiveTick`
  (params (DeltaSeconds :type "Float (single-precision)"))
  (bind _returnvalue (`GameplayStatics.GetPlayerController` 0))
  (bind _asfisticuffs_game_mode (cast `FisticuffsGameMode` (`GameplayStatics.GetGameMode`)))
  (if (`|EnumEquality` (`FisticuffsGameMode.PlayState` _asfisticuffs_game_mode) "EMainMenu")
    (set `PlayerController.bShowMouseCursor` true _returnvalue)
    (else
      (`SceneComponent.SetHiddenInGame` true true)
      (set `PlayerController.bShowMouseCursor` false _returnvalue))))

(fn `UserConstructionScript`)