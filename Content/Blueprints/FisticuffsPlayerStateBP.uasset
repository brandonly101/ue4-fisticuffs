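; Player state for a fistfighting game that mirrors the player fighter's current discombobulation and stamina stats.
; On BeginPlay and every Tick it casts player pawn 0 to FistFighterBP and copies both values into its own variables.
; The pawn is looked up by index 0 rather than through the owning player, so the values always reflect that pawn.
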(event `self.ReceiveBeginPlay`
  (`parent.ReceiveBeginPlay`)
  (bind _asfist_fighter_bp (cast `/Game/Blueprints/PlayerCharacterBP/FistFighterBP` (`GameplayStatics.GetPlayerPawn` 0)))
  (set `self.FighterStatDiscombobCurrent` (`/Game/Blueprints/PlayerCharacterBP/FistFighterBP.StatDiscombobulation` _asfist_fighter_bp))
  (set `self.FighterStatStaminaCurrent` (`/Game/Blueprints/PlayerCharacterBP/FistFighterBP.StatStamina` _asfist_fighter_bp)))

(event `self.ReceiveTick`
  (params (DeltaSeconds :type "Float (single-precision)"))
  (`parent.ReceiveTick` DeltaSeconds)
  (bind _asfist_fighter_bp (cast `/Game/Blueprints/PlayerCharacterBP/FistFighterBP` (`GameplayStatics.GetPlayerPawn` 0)))
  (set `self.FighterStatDiscombobCurrent` (`/Game/Blueprints/PlayerCharacterBP/FistFighterBP.StatDiscombobulation` _asfist_fighter_bp))
  (set `self.FighterStatStaminaCurrent` (`/Game/Blueprints/PlayerCharacterBP/FistFighterBP.StatStamina` _asfist_fighter_bp)))

(fn `UserConstructionScript`)