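; Utility Blueprint of common helper functions for timers and random values.
; Timer is an unfinished test that sets a fixed timer with no function name, then immediately clears TimerDispatch, leaving its randomized duration unused.
; TimerDispatch only prints a test string.
; RandomValue returns a float in a range from a random stream seeded by the current clock millisecond.
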(fn `RandomValue`
  (params (Min :type "Float (double-precision)" :default 0.0) (Max :type "Float (double-precision)"))
  (returns (`Random Value` :type "Float (double-precision)"))
  (return (`KismetMathLibrary.RandomFloatInRangeFromStream` Min Max (`KismetMathLibrary.MakeRandomStream` (`KismetMathLibrary.GetMillisecond` (`KismetMathLibrary.Now`))))))

(fn `Timer`
  (params (TimerConstant :type "Float (double-precision)" :default 0.0) (TimerRange :type "Float (double-precision)" :default 0.0))
  (`|ExecutionSequence`
    (:`then_0`
      (`KismetSystemLibrary.K2_SetTimer` null "" 3.0))
    (:`then_1`
      (`KismetSystemLibrary.K2_ClearTimer` null "TimerDispatch"))))

(fn `TimerDispatch`
  (`KismetSystemLibrary.PrintString` null "TImer Test"))